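; ZD_Player_Lobby is the player actor for the lobby, displaying that player's lobby info through a widget component.
; UpdatePlayerLobbyInfo sets the PlayerLobbyInfo variable, whose RepNotify pushes it into the WB_PlayerLobbyInfo widget and shows the component, retrying on a short timer until the widget is valid.
; UpdateRotation snaps the control rotation to face one of two opposite yaw directions based on the sign of a non-zero direction input.
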(fn `OnRep_PlayerLobbyInfo`
  (bind _returnvalue (`WidgetComponent.GetWidget` (`self.LobbyInfo1`)))
  (`/Engine/EditorBlueprintResources/StandardMacros.IsValid` _returnvalue
    (:`Is Valid`
      (bind _aswb_player_lobby_info (cast `/Game/Lobby/Blueprints/Lobby/WB_PlayerLobbyInfo` _returnvalue))
      (`/Game/Lobby/Blueprints/Lobby/WB_PlayerLobbyInfo.Update` _aswb_player_lobby_info (`self.PlayerLobbyInfo`))
      (`SceneComponent.SetVisibility` (`self.LobbyInfo1`) true false))
    (:`Is Not Valid`
      (`KismetSystemLibrary.K2_SetTimer` null "OnRep_PlayerLobbyInfo" 0.1))))

(fn `UpdatePlayerLobbyInfo`
  (params (PlayerLobbyInfo :type "/Game/Lobby/Blueprints/Lobby/S_PlayerLobbyInfo Structure"))
  (set `self.PlayerLobbyInfo` PlayerLobbyInfo))

(fn `UpdateRotation`
  (params (Direction :type "Float (double-precision)"))
  (if (!= Direction 0.0)
    (`Controller.SetControlRotation` (`self.GetController`) (select `bool` (>= Direction 0.0) :`false` (`KismetMathLibrary.MakeRotator` 0.0 0.0 180.0) :`true` (`KismetMathLibrary.MakeRotator` 0.0)))))

(fn `UserConstructionScript`)