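; Pressure button that moves a linked MovableObject along a chosen axis when a ZD_Player_BASE steps on or off it.
; Box overlap or debug E key plays press/release timelines that slide the Cylinder, then fire PressedButton or ReleasedButton.
; Those events run further timelines into per-axis move functions, gated by ObjectMoved.
; MoveOnY lerps from the transform cached at BeginPlay, while X and Z offset the current transform each update, so movement compounds.
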(event OnComponentBeginOverlap(Box)
  (params (OverlappedComponent :type Primitive%20Component%20Object%20Reference) (OtherActor :type Actor%20Object%20Reference) (OtherComp :type Primitive%20Component%20Object%20Reference) (OtherBodyIndex :type Integer) (bFromSweep :type Boolean) (SweepResult :type Hit%20Result%20Structure%20%28by%20ref%29))
  (bind _cylinder (Variables|Default|GetCylinder))
  (Utilities|Casting|CastToZD_Player_BASE OtherActor)
  (bind _pressbutton (Timeline|PressButton PlayFromStart)
    (:Update
      (Transformation|SetRelativeLocation _cylinder (Math|Vector|MakeVector 0.0 0.0 (Math|Float|Lerp (.z (Variables|/Script/Engine.SceneComponent|GetRelativeLocation _cylinder)) -1e+01 _pressbutton)) false false))
    (:Finished
      (CallFunction|PressedButton))))

(event OnComponentEndOverlap(Box)
  (params (OverlappedComponent :type Primitive%20Component%20Object%20Reference) (OtherActor :type Actor%20Object%20Reference) (OtherComp :type Primitive%20Component%20Object%20Reference) (OtherBodyIndex :type Integer))
  (bind _cylinder (Variables|Default|GetCylinder))
  (Utilities|Casting|CastToZD_Player_BASE OtherActor)
  (bind _releasebutton (Timeline|ReleaseButton PlayFromStart)
    (:Update
      (Transformation|SetRelativeLocation _cylinder (Math|Vector|MakeVector 0.0 0.0 (Math|Float|Lerp (.z (Variables|/Script/Engine.SceneComponent|GetRelativeLocation _cylinder)) 0.0 _releasebutton)) false false))
    (:Finished
      (CallFunction|ReleasedButton))))

(event Custom|PressedButton
  (bind _movableobject (Variables|Default|GetMovableObject))
  (if (not (Variables|Default|GetObjectMoved))
    (bind _pressbutton (Timeline|Timeline PlayFromStart)
      (:Update
        (switch Utilities|FlowControl|Switch|SwitchonE_ButtonOptions (Variables|Default|GetObjectMoveOptions)
          (:NewEnumerator0
            (CallFunction|MoveonX _movableobject _pressbutton false))
          (:NewEnumerator1
            (CallFunction|MoveonY _movableobject _pressbutton false))
          (:NewEnumerator2
            (CallFunction|MoveonZ _movableobject _pressbutton false)))
        (Variables|Default|SetObjectMoved true)))))

(event Custom|ReleasedButton
  (bind _movableobject (Variables|Default|GetMovableObject))
  (if (Variables|Default|GetObjectMoved)
    (bind _releasebutton (Timeline|Timeline_0 PlayFromStart)
      (:Update
        (switch Utilities|FlowControl|Switch|SwitchonE_ButtonOptions (Variables|Default|GetObjectMoveOptions)
          (:NewEnumerator0
            (CallFunction|MoveonX _movableobject _releasebutton true))
          (:NewEnumerator1
            (CallFunction|MoveonY _movableobject _releasebutton true))
          (:NewEnumerator2
            (CallFunction|MoveonZ _movableobject _releasebutton true)))
        (Variables|Default|SetObjectMoved false)))))

(event Collision|EventActorBeginOverlap
  (params (OtherActor :type Actor%20Object%20Reference)))

(event EventTick
  (params (DeltaSeconds :type Float%20%28single-precision%29)))

(event EventBeginPlay
  (Variables|Default|SetBaseObjectTransform (Transformation|GetActorTransform (Variables|Default|GetMovableObject))))

(event Input|KeyboardEvents|DebugKeyE
  (params (Key :type Key%20Structure) (ActionValue :type Input%20Action%20Value%20Structure))
  (bind _cylinder (Variables|Default|GetCylinder))
  (bind _cylinder_2 (Variables|Default|GetCylinder))
  (:Pressed
    (bind _pressbutton (Timeline|PressButton PlayFromStart)
      (:Update
        (Transformation|SetRelativeLocation _cylinder_2 (Math|Vector|MakeVector 0.0 0.0 (Math|Float|Lerp (.z (Variables|/Script/Engine.SceneComponent|GetRelativeLocation _cylinder_2)) -1e+01 _pressbutton)) false false))
      (:Finished
        (CallFunction|PressedButton))))
  (:Released
    (bind _releasebutton (Timeline|ReleaseButton PlayFromStart)
      (:Update
        (Transformation|SetRelativeLocation _cylinder (Math|Vector|MakeVector 0.0 0.0 (Math|Float|Lerp (.z (Variables|/Script/Engine.SceneComponent|GetRelativeLocation _cylinder)) 0.0 _releasebutton)) false false))
      (:Finished
        (CallFunction|ReleasedButton)))))

(fn ConstructionScript)

(fn MoveonX
  (params (self2 :type Actor%20Object%20Reference) (Alpha :type Float%20%28double-precision%29) (ReverseMoveObject :type Boolean))
  (bind _returnvalue (Transformation|GetActorTransform self2))
  (bind _returnvalue_2 (Transformation|GetActorTransform self2))
  (if (not ReverseMoveObject)
    (Transformation|SetActorRelativeTransform self2 (Math|Transform|MakeTransform (Math|Vector|MakeVector (Math|Float|Lerp (.x (.location _returnvalue_2)) (+ (.x (.location _returnvalue_2)) (Variables|Default|GetMovableObjectMoveDistance)) Alpha) (.y (.location _returnvalue_2)) (.z (.location _returnvalue_2))) (.rotation _returnvalue_2) (.scale _returnvalue_2)) false false)
    (else
      (Transformation|SetActorRelativeTransform self2 (Math|Transform|MakeTransform (Math|Vector|MakeVector (Math|Float|Lerp (.x (.location _returnvalue)) (- (.x (.location _returnvalue)) (Variables|Default|GetMovableObjectMoveDistance)) Alpha) (.y (.location _returnvalue)) (.z (.location _returnvalue))) (.rotation _returnvalue) (.scale _returnvalue)) false false))))

(fn MoveonY
  (params (self2 :type Actor%20Object%20Reference) (Alpha :type Float%20%28double-precision%29) (ReverseMoveObject :type Boolean))
  (bind _movableobjectmovedistance (Variables|Default|GetMovableObjectMoveDistance))
  (bind _baseobjecttransform (Variables|Default|GetBaseObjectTransform))
  (bind _baseobjecttransform_2 (Variables|Default|GetBaseObjectTransform))
  (bind _returnvalue (+ (.y (.location _baseobjecttransform_2)) _movableobjectmovedistance))
  (bind _returnvalue_2 (Math|Float|Lerp (.y (.location _baseobjecttransform_2)) _returnvalue Alpha))
  (if (not ReverseMoveObject)
    (Variables|Default|SetUpdatedObjectTransform (Math|Transform|MakeTransform (Math|Vector|MakeVector (.x (.location _baseobjecttransform_2)) _returnvalue_2 (.z (.location _baseobjecttransform_2))) (.rotation _baseobjecttransform_2) (.scale _baseobjecttransform_2)))
    (Transformation|SetActorRelativeTransform self2 (Math|Transform|MakeTransform (Math|Vector|MakeVector (.x (.location _baseobjecttransform_2)) _returnvalue_2 (.z (.location _baseobjecttransform_2))) (.rotation _baseobjecttransform_2) (.scale _baseobjecttransform_2)) false false)
    (else
      (Transformation|SetActorRelativeTransform self2 (Math|Transform|MakeTransform (Math|Vector|MakeVector (.x (.location _baseobjecttransform)) (Math|Float|Lerp (.y (.location _baseobjecttransform)) (.y (.location (Variables|Default|GetUpdatedObjectTransform))) Alpha) (.z (.location _baseobjecttransform))) (.rotation _baseobjecttransform) (.scale _baseobjecttransform)) false false))))

(fn MoveonZ
  (params (self2 :type Actor%20Object%20Reference) (Alpha :type Float%20%28double-precision%29) (ReverseObjectMove :type Boolean))
  (bind _returnvalue (Transformation|GetActorTransform self2))
  (bind _returnvalue_2 (Transformation|GetActorTransform self2))
  (if (not ReverseObjectMove)
    (Transformation|SetActorRelativeTransform self2 (Math|Transform|MakeTransform (Math|Vector|MakeVector (.x (.location _returnvalue_2)) (.y (.location _returnvalue_2)) (Math|Float|Lerp (.z (.location _returnvalue_2)) (+ (.z (.location _returnvalue_2)) (Variables|Default|GetMovableObjectMoveDistance)) Alpha)) (.rotation _returnvalue_2) (.scale _returnvalue_2)) false false)
    (else
      (Transformation|SetActorRelativeTransform self2 (Math|Transform|MakeTransform (Math|Vector|MakeVector (.x (.location _returnvalue)) (.y (.location _returnvalue)) (Math|Float|Lerp (.z (.location _returnvalue)) (- (.z (.location _returnvalue)) (Variables|Default|GetMovableObjectMoveDistance)) Alpha)) (.rotation _returnvalue) (.scale _returnvalue)) false false))))