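; Game instance Blueprint that hosts multiplayer sessions and handles accepted session invites.
; CreateSession creates an advanced session for the first player, then opens the Lobby level as a listen server on success.
; An accepted invite destroys any current session, then joins the invited one whether or not the destroy succeeds, printing debug messages along the way.
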(event `CreateSession`
  (`CreateSessionCallbackProxyAdvanced.CreateAdvancedSession` :`PlayerController` (`GameplayStatics.GetPlayerController` 0)
    (:`OnSuccess`
      (`GameplayStatics.OpenLevelBySoftObjectPtr` "/Game/Lobby/Maps/Lobby.Lobby" true "listen"))))

(event `self.OnSessionInviteAccepted`
  (params (LocalPlayerNum :type Integer) (PersonInvited :type "BPUniqueNetId Structure") (SessionToJoin :type "BlueprintSessionResult Structure (by ref)"))
  (bind _returnvalue (`GameplayStatics.GetPlayerController` 0))
  (`KismetSystemLibrary.PrintString` (`AdvancedSessionsLibrary.GetSessionID_AsString` SessionToJoin))
  (`KismetSystemLibrary.PrintString` (`KismetSystemLibrary.GetDisplayName` _returnvalue))
  (`DestroySessionCallbackProxy.DestroySession` _returnvalue
    (:`OnSuccess`
      _)
    (:`OnFailure`
      _))
  (`JoinSessionCallbackProxy.JoinSession` _returnvalue SessionToJoin
    (:`OnSuccess`
      (`KismetSystemLibrary.PrintString` "Joined Session"))
    (:`OnFailure`
      (`KismetSystemLibrary.PrintString` "Failed To Join"))))