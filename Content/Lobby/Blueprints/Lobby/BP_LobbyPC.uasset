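; Lobby player controller that manages a player's ready status and lobby UI.
; For the local player it creates the lobby widget with a mouse cursor and game-and-UI input.
; It passes itself to BP_LobbyGM to update lobby info on BeginPlay, on ready toggles (also bound to a debug key) and via a delayed retry event.
; On match start it shows the loading screen and disables input.
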(event Custom|TryAgainUpdatingLobbyInfo
  (Utilities|FlowControl|Delay 0.1)
  (bind _asbp_lobby_gm (Utilities|Casting|CastToBP_LobbyGM (Game|GetGameMode)))
  (Default|UpdatePlayerLobbyInfo _asbp_lobby_gm self))

(event Custom|ToggleReadyStatusOnServer
  (bind _playerlobbyinfopc (Variables|Default|GetPlayerLobbyInfoPC))
  (Utilities|Struct|SetmembersinS_PlayerLobbyInfo _playerlobbyinfopc (not (.bReady (Utilities|Struct|BreakS_PlayerLobbyInfo _playerlobbyinfopc))))
  (bind _asbp_lobby_gm (Utilities|Casting|CastToBP_LobbyGM (Game|GetGameMode)))
  (Default|UpdatePlayerLobbyInfo _asbp_lobby_gm self))

(event Custom|OnStartMatch
  (Default|ShowLoadingScreen (Variables|Default|GetLobbyUI_Ref))
  (Input|DisableInput self))

(event EventBeginPlay
  (CallFunction|SetUp)
  (bind _asbp_lobby_gm (Utilities|Casting|CastToBP_LobbyGM (Game|GetGameMode)))
  (Default|UpdatePlayerLobbyInfo _asbp_lobby_gm self))

(event EventTick
  (params (DeltaSeconds :type Float%20%28single-precision%29)))

(event Input|KeyboardEvents|DebugKeyR
  (params (Key :type Key%20Structure) (ActionValue :type Input%20Action%20Value%20Structure))
  (:Pressed
    (CallFunction|ToggleReadyStatusonServer)))

(fn ConstructionScript)

(fn SetUp
  (if (Pawn|IsLocalPlayerController)
    (Variables|Default|SetbShowMouseCursor true)
    (Input|SetInputModeGameandUI self 0 "DoNotLock" false false)
    (bind _returnvalue (UserInterface|CreateWidget "/Game/Lobby/Blueprints/Lobby/WB_LobbyUI.WB_LobbyUI_C"))
    (bind _output_get (Variables|Default|SetLobbyUI_Ref _returnvalue))
    (UserInterface|Viewport|AddtoViewport _output_get 0)))